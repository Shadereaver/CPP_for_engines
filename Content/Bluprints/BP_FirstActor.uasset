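; BP_FirstActor is an actor that plays a repeating 2D hi-hat sound as a Quartz-driven metronome.
; On BeginPlay it creates a 4/4 Quartz clock, sets a fixed tempo and subscribes to quarter-note quantization events, then starts the clock after a short delay.
; Each quantization event fires the Hihat handler, so the sound follows the audio clock's timing rather than Tick.
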(event Custom|Hihat
  (params (ClockName :type Name) (QuantizationType :type EQuartzCommandQuantization%20Enum :default "Bar") (NumBars :type Integer) (Beat :type Integer) (BeatFraction :type Float%20%28single-precision%29))
  (Audio|PlaySound2D "/Game/Audio/Hihat.Hihat" 1.0 1.0 0.0 0 0))

(event EventBeginPlay
  (bind _returnvalue (Class|QuartzSubsystem|CreateNewClock (WorldSubsystems|GetQuartzSubsystem) "Hi" (Utilities|Struct|MakeQuartzClockSettings (Utilities|Struct|MakeQuartzTimeSignature 4 "QuarterNote") false) false))
  (bind _output_get (Variables|Default|SetClock_hi _returnvalue))
  (bind _clockhandle (Class|QuartzClockHandle|SetBeatsPerMinute :self _output_get :BeatsPerMinute 1.8e+02))
  (bind _clockhandle_2 (Class|QuartzClockHandle|SubscribetoQuantizationEvent _clockhandle "QuarterNote" (delegate Custom|Hihat)))
  (Utilities|FlowControl|Delay 1.0)
  (Class|QuartzClockHandle|StartClock _clockhandle_2))

(fn ConstructionScript)